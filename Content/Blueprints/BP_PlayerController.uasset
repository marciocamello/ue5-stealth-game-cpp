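; Player controller that shows the game instructions screen and the end-of-mission screen.
; BeginPlay creates the W_StartGame widget, and Tab alternates between removing it and creating it again through a FlipFlop.
; Both paths branch on authority, with server-named wrapper events forwarding to the client-side widget events.
; OnMissionCompleted adds a W_GameOver widget, passing it the mission success result.
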(event Custom|InitGameInstrunctions
  ;[1 1 1] Client functions
  (bind _returnvalue (UserInterface|CreateWidget "/Game/UI/W_StartGame.W_StartGame_C" (Game|GetPlayerController 0)))
  (bind _output_get (Variables|Default|SetW_StartGame _returnvalue))
  (UserInterface|Viewport|AddtoViewport _output_get 0))

(event Custom|InitGameInstrunctions_Server
  ;[1 1 1] Server functions
  (CallFunction|InitGameInstrunctions))

(event Custom|StartGame
  ;[1 1 1] Client functions
  (Widget|RemovefromParent (Variables|Default|GetW_StartGame)))

(event Custom|StartGame_Server
  ;[1 1 1] Server functions
  (CallFunction|StartGame))

(event EventBeginPlay
  (if (Ability|HasAuthority)
    (CallFunction|InitGameInstrunctionsServer)
    (else
      (CallFunction|InitGameInstrunctions))))

(event EventOnMissionCompleted
  (params (InstigatorPawn :type Pawn%20Object%20Reference) (bMissionSuccess :type Boolean))
  ;[1 1 1] Show widget with game over or mission is completed
  (bind _returnvalue (UserInterface|CreateWidget "/Game/UI/W_GameOver.W_GameOver_C" 0 bMissionSuccess))
  (UserInterface|Viewport|AddtoViewport _returnvalue 0))

(event Input|KeyboardEvents|Tab
  (params (Key :type Key%20Structure :default "None"))
  ;[1 1 1] Toggle StartGame and Show instructions
  (:Pressed
    (Utilities|FlowControl|FlipFlop
      (:A
        (if (Ability|HasAuthority)
          (CallFunction|StartGameServer)
          (else
            (CallFunction|StartGame))))
      (:B
        (if (Ability|HasAuthority)
          (CallFunction|InitGameInstrunctionsServer)
          (else
            (CallFunction|InitGameInstrunctions)))))))

(fn ConstructionScript)