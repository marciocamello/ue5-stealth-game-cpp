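; BP_LaunchPad is a launch pad that throws characters and physics objects that overlap it.
; On overlap, it builds a velocity from the actor's forward direction, pitched by a launch angle and scaled by a strength value.
; Characters are launched with both XY and Z velocity overridden, while other physics-simulating components receive a mass-independent velocity-change impulse.
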(event OnComponentBeginOverlap(OverlapComp)
  (params (OverlappedComponent :type Primitive%20Component%20Object%20Reference) (OtherActor :type Actor%20Object%20Reference) (OtherComp :type Primitive%20Component%20Object%20Reference) (OtherBodyIndex :type Integer) (bFromSweep :type Boolean) (SweepResult :type Hit%20Result%20Structure%20%28by%20ref%29))
  (bind _returnvalue (Transformation|GetActorRotation))
  (bind (_roll _pitch _yaw) (Math|Rotator|BreakRotator _returnvalue))
  (Variables|Default|SetLaunchVelocity (* (Math|Vector|GetForwardVector (Math|Rotator|MakeRotator _roll (+ _pitch (Variables|Default|GetLaunchPitchAngle)) _yaw)) (Variables|Default|GetLaunchStrength)))
  (bind _ascharacter (Utilities|Casting|CastToCharacter OtherActor)
    (:then
      (Utilities|IsValid _ascharacter
        (:Is%20Valid
          (Character|LaunchCharacter _ascharacter (Variables|Default|GetLaunchVelocity) true true))))
    (:CastFailed
      (Utilities|IsValid OtherComp
        (:Is%20Valid
          (if (Physics|IsSimulatingPhysics OtherComp "None")
            (Physics|AddImpulse OtherComp (Variables|Default|GetLaunchVelocity) "None" true)))))))

(fn ConstructionScript)